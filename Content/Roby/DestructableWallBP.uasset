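; DestructableWallBP is a wall that catches fire when an AI_Character overlaps its FireTrigger and breaks if left burning.
; SetOnFire activates the particle system and starts a timer that calls DestroyWall by function name.
; An overlapping Projectile_Master_BP extinguishes it, stopping the particles and clearing that timer.
; DestroyWall swaps the intact mesh for the broken one, hidden at construction, and disables the intact wall's collider.
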(event `self.ReceiveBeginPlay`)

(event `self.ReceiveActorBeginOverlap`
  (params (OtherActor :type "Actor Object Reference")))

(event `self.Fire Trigger.OnComponentBeginOverlap`
  (params (OtherActor :type "Actor Object Reference") (OtherComp :type "PrimitiveComponent Object Reference") (OtherBodyIndex :type Integer) (bFromSweep :type Boolean) (SweepResult :type "HitResult Structure (by ref)"))
  (`|ExecutionSequence`
    (:`then_0`
      (cast `/Game/AI/AI_Character` OtherActor)
      (`self.SetOnFire`))
    (:`then_1`
      (cast `/Game/Roby/Projectile_Master_BP` OtherActor)
      (`self.Extinguish`))))

(event `self.ReceiveTick`
  (params (DeltaSeconds :type "Float (single-precision)")))

(fn `DestroyWall`
  (`SceneComponent.SetVisibility` (`self.BrokenMesh`) true true)
  (`SceneComponent.SetVisibility` (`self.NormalWall`) false true)
  (`PrimitiveComponent.SetCollisionEnabled` (`self.NormalWallCollider`) "NoCollision"))

(fn `Extinguish`
  (`ActorComponent.Deactivate` (`self.ParticleSystem`))
  (`KismetSystemLibrary.K2_ClearTimerHandle` (`self.TimerHandle`)))

(fn `SetOnFire`
  (`ActorComponent.Activate` (`self.ParticleSystem`) false)
  (bind _returnvalue (`KismetSystemLibrary.K2_SetTimer` null "DestroyWall" 20.0))
  (set `self.TimerHandle` _returnvalue))

(fn `UserConstructionScript`
  (`SceneComponent.SetVisibility` (`self.BrokenMesh`) false true))