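; Master Blueprint for a flammable object that AI characters ignite and projectiles extinguish in a firefighting game.
; FireTrigger overlaps drive it: AI starts fire particles, sound and a destruction timer, while a burning object sets the player on fire.
; Projectile hits stop the fire, clear the timer and add SaveValue through the game mode's UpdateScore.
; On timer expiry it ignores further overlaps, blackens its dynamic material and switches particles to smoke.
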(event `self.ReceiveBeginPlay`)

(event `self.ReceiveActorBeginOverlap`
  (params (OtherActor :type "Actor Object Reference")))

(event `self.ReceiveTick`
  (params (DeltaSeconds :type "Float (single-precision)")))

(event `self.Fire Trigger.OnComponentBeginOverlap`
  (params (OtherActor :type "Actor Object Reference") (OtherComp :type "PrimitiveComponent Object Reference") (OtherBodyIndex :type Integer) (bFromSweep :type Boolean) (SweepResult :type "HitResult Structure (by ref)"))
  ;[1 1 1] Implement Player Damage and Enemy
  (if (not (`self.Destroyed`))
    (`|ExecutionSequence`
      (:`then_0`
        (bind _asthird_person_character (cast `/Game/ThirdPersonBP/Blueprints/ThirdPersonCharacter` OtherActor))
        (if (`self.OnFire`)
          (`/Game/ThirdPersonBP/Blueprints/ThirdPersonCharacter.SetOnFire` _asthird_person_character)))
      (:`then_1`
        (cast `/Game/Roby/Projectile_Master_BP` OtherActor)
        (`self.StopFire`))
      (:`then_2`
        (cast `/Game/AI/AI_Character` OtherActor)
        (`self.StartFire`)
        (`KismetSystemLibrary.PrintString` "I'm On FIreee")
        (bind _returnvalue (`KismetSystemLibrary.K2_SetTimer` null "DestroyMe" 10.0))
        (set `self.DestructionTImer` _returnvalue)))))

(fn `DestroyMe`
  (set `self.Destroyed` true)
  (`MaterialInstanceDynamic.SetVectorParameterValue` :`self` (`self.BurntMaterial`) :`ParameterName` "BodyColor")
  (`ParticleSystemComponent.SetTemplate` (`self.ParticleSystem`) "/Game/StarterContent/Particles/P_Smoke.P_Smoke"))

(fn `StartFire`
  ;[1 1 1] Create the scale up effect
  (set `self.OnFire` true)
  (`ActorComponent.Activate` (`self.ParticleSystem`) false)
  (`GameplayStatics.PlaySoundAtLocation` "/Game/StarterContent/Audio/Fire01.Fire01" (`self.K2_GetActorLocation`)) ; Play firing sound
)

(fn `StopFire`
  (set `self.OnFire` false)
  (`ActorComponent.Deactivate` (`self.ParticleSystem`))
  (`KismetSystemLibrary.K2_ClearTimerHandle` (`self.DestructionTImer`))
  (bind _asfire_fighting_game_mode (cast `/Game/Roby/FireFIghtingGameMode` (`GameplayStatics.GetGameMode`)))
  (`/Game/Roby/FireFIghtingGameMode.UpdateScore` _asfire_fighting_game_mode (`self.SaveValue`)))

(fn `UserConstructionScript`
  (bind _mesh (`self.Mesh`))
  (bind _returnvalue (`PrimitiveComponent.CreateDynamicMaterialInstance` _mesh 0 (`KismetArrayLibrary.Array_Get` (`MeshComponent.GetMaterials` _mesh))))
  (set `self.BurntMaterial` _returnvalue))